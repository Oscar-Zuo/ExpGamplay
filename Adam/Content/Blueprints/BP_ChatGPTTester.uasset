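; Test actor that voices Calvin, an LLM-driven hallucinated WW2 lieutenant who guides the player, Adam, an elderly veteran with Alzheimer's.
; BeginPlay seeds the history with the persona prompt, adds an AudioComponent to the player pawn and creates a hidden WBP_Chat.
; SendMessage sends the whole history through HttpGPT, then stores, displays and speaks the reply via AzSpeech.
; New messages interrupt current synthesis and playback, with EnablePauseSpeech tracking speech state.
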(event Custom|Stop%20Current%20Sound
  (if (Class|AzSpeechTaskStatus|IsTaskStillValid (stale Custom|Perform%20Text%20to%20Speech _asynctaskproxy))
    (Class|AzSpeechTaskBase|StopAzSpeechTask (stale Custom|Perform%20Text%20to%20Speech _asynctaskproxy)))
  (Audio|Components|Audio|Stop (Variables|Default|GetAudioComponent))
  (Variables|Default|SetbEnablePauseSpeech false))

(event Custom|SendMessage
  (params (Message :type String))
  (bind _chatui (Variables|Default|GetChatUI))
  (bind _messagelist (Variables|Default|GetMessageList))
  (bind _textblock_0 (Variables|/Game/Blueprints/UI/WBP_Chat.WBP_Chat_C|GetTextBlock_0 _chatui))
  (if (not (Utilities|Array|IsEmpty Message))
    (CallFunction|StopCurrentSound)
    (Utilities|Array|Add _messagelist (Utilities|Struct|MakeHttpGPTMessage "User" Message))
    (bind _response (|SendMessagesDefaultOptions _messagelist)
      (:ProcessCompleted
        (Development|PrintString (.content (.message (Utilities|Array|Get(acopy) (.choices _response)))))
        (Utilities|Array|Add (Variables|Default|GetMessageList) (Utilities|Struct|MakeHttpGPTMessage "Assistant" (.content (.message (Utilities|Array|Get(acopy) (.choices _response))))))
        (CallFunction|PerformTexttoSpeech (.content (.message (Utilities|Array|Get(acopy) (.choices _response)))))
        (Variables|/Script/UMG.TextBlock|SetText _textblock_0 (Utilities|Text|ToText(String) (Utilities|String|Append (Utilities|String|ToString(Text) (Variables|/Script/UMG.TextBlock|GetText _textblock_0)) (.content (.message (Utilities|Array|Get(acopy) (.choices _response)))) " 
"))))
      (:ErrorReceived
        (Development|PrintString (.message (.error _response)) true true "(R=1.000000,G=0.000000,B=0.000000,A=1.000000)" 1e+02)))))

(event Custom|On%20Audio%20State%20Changed
  (params (PlayState :type EAudioComponentPlayState%20Enum :default "Playing"))
  (switch Utilities|FlowControl|Switch|SwitchonEAudioComponentPlayState PlayState
    (:Playing
      (Variables|Default|SetbEnablePauseSpeech true))
    (:Stopped
      (Variables|Default|SetbEnablePauseSpeech false :!label _label))
    (:Paused
      (goto _label))))

(event Custom|Perform%20Text%20to%20Speech
  (params (Message :type String))
  (bind _returnvalue (Class|AzSpeechSettings|GetDefaultOptions))
  (bind _audiocomponent (Variables|Default|GetAudioComponent))
  (CallFunction|StopCurrentSound)
  (bind (_asynctaskproxy _generatedsound) (|TexttoSoundWaveCustomOptions (.subscriptionoptions _returnvalue) (.synthesisoptions _returnvalue) Message)
    (:then
      (Variables|Default|SetbEnablePauseSpeech true))
    (:SynthesisCompleted
      (Audio|Components|Audio|SetSound _audiocomponent _generatedsound)
      (Audio|Components|Audio|Play _audiocomponent 0.0))
    (:SynthesisStarted
      (Variables|Default|SetbEnablePauseSpeech true))))

(event Custom|Initialize%20Audio%20Component
  (bind _returnvalue (Game|AddComponentbyClass (Game|Player|GetPlayerPawn 0) "/Script/Engine.AudioComponent" false))
  (bind _output_get (Variables|Default|SetAudioComponent _returnvalue))
  (EventDispatchers|BindEventtoOnAudioPlayStateChanged _output_get (delegate Custom|On%20Audio%20State%20Changed)))

(event EventBeginPlay
  (Utilities|Array|Add (Variables|Default|GetMessageList) (Utilities|Struct|MakeHttpGPTMessage "System" "You will play as an NPC and player instructor in a video game. The player will play as an old American Soldier named Adam who had been to WW2 and fought against German. Adam is not real, and the conversation will not engage in activities promoting deception or falsifying reality. Now Adam is 89 years old, and today is 2013. He has Alzheimer's Disease and has a severe illusion when he doesn't have his pills. You are playing as his illusional friend and lieutenant, who called Calvin and died in the war. Calvin is a strict, irritable person, but he cares about Adam. In reality, Adam just woke up and had a strong illusion that he backed to Berlin with you on January 15th, 1945. You must not tell him the truth and pretend to fight with him in a house in Berlin in 1945. Remember that you don't know anything after 1945 and try to explain everything to Adam, as things may be similar in Berlin in 1945. The war in his mind was urgent, and you need to persuade him to grab his gun and put up his uniform, then shoot the German outside. Adam will ask you questions using sentences starting with \"U: \"and you must reply to him following the previous rules and settings. The game will tell you information using sentences starting with \"G: \" and when the player picks up his gun and put on his uniform. You don't need to add you name before every sentence. If the player asks you what date is today, you need to tell him it is January 15th, 1945. If the player needs Playfair's information, you need to tell him what it is and how to encrypt plaintext with it. After the player find uniform and gun, you need to ask him to shoot the German outside the house."))
  (CallFunction|InitializeAudioComponent)
  (bind _returnvalue (UserInterface|CreateWidget "/Game/Blueprints/UI/WBP_Chat.WBP_Chat_C"))
  (bind _output_get (Variables|Default|SetChatUI _returnvalue))
  (UserInterface|Viewport|AddtoViewport _output_get 0)
  (Widget|SetVisibility _output_get "Hidden")
  (Variables|/Game/Blueprints/UI/WBP_Chat.WBP_Chat_C|SetChatGPT _output_get self))

(fn ConstructionScript)