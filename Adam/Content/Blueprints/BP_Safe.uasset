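; Interactable safe actor that shows a keypad-style panel and swings open when Open is called.
; Trigger, if not already Opened, creates WBP_SafePannel with a reference to itself, shows the cursor and disables first-person character input.
; Open yaws the whole actor up to 90 degrees via a timeline, removes the panel and restores cursor and input state.
; Opened is checked but never set in these graphs.
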(event Custom|Open
  (Utilities|FlowControl|Sequence
    (:then_0
      (bind _output_get (Variables|Default|SetOriginalRotation (Transformation|GetActorRotation)))
      (bind _newtrack_0 (Timeline|DoorTimeLine Play)
        (:Update
          (Transformation|SetActorRotation (Math|Rotator|MakeRotator (.roll _output_get) (.pitch _output_get) (+ (.yaw _output_get) (* _newtrack_0 9e+01)))))))
    (:then_1
      (Widget|RemovefromParent (Variables|Default|GetPanelUI))
      (Variables|/Script/Engine.PlayerController|SetbShowMouseCursor (Game|GetPlayerController 0) false)
      (bind _asbp_first_person_character (Utilities|Casting|CastToBP_FirstPersonCharacter (Game|GetPlayerCharacter 0)))
      (Variables|/Game/FirstPerson/Blueprints/BP_FirstPersonCharacter.BP_FirstPersonCharacter_C|SetCanInput _asbp_first_person_character true))))

(event EventBeginPlay)

(event Collision|EventActorBeginOverlap
  (params (OtherActor :type Actor%20Object%20Reference)))

(event EventTick
  (params (DeltaSeconds :type Float%20%28single-precision%29)))

(event EventTrigger
  (params (Player :type BP%20First%20Person%20Character%20Object%20Reference))
  (if (not (Variables|Default|GetOpened))
    (bind _returnvalue (UserInterface|CreateWidget "/Game/Blueprints/UI/WBP_SafePannel.WBP_SafePannel_C"))
    (bind _output_get (Variables|Default|SetPanelUI _returnvalue))
    (UserInterface|Viewport|AddtoViewport _output_get 0)
    (Variables|/Script/Engine.PlayerController|SetbShowMouseCursor (Game|GetPlayerController 0) true)
    (Variables|/Game/Blueprints/UI/WBP_SafePannel.WBP_SafePannel_C|SetSafe _returnvalue self)
    (bind _asbp_first_person_character (Utilities|Casting|CastToBP_FirstPersonCharacter (Game|GetPlayerCharacter 0)))
    (Variables|/Game/FirstPerson/Blueprints/BP_FirstPersonCharacter.BP_FirstPersonCharacter_C|SetCanInput _asbp_first_person_character false)))

(fn ConstructionScript)