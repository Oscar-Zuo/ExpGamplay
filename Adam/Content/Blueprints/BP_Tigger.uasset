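; BP_Tigger is a Blueprint trigger that sends the player to the "Reality" level.
; Its Trigger event takes a Player and opens that level by name only when the player has both the rifle and the uniform.
; BeginPlay, overlap and Tick are disabled stubs, so the check runs only when Trigger is called from outside this graph.
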(event EventBeginPlay
  (|CallParentFunction) ; This node is disabled and will not be called.\nDrag off pins to build functionality.
)

(event Collision|EventActorBeginOverlap
  (params (OtherActor :type Actor%20Object%20Reference))
  (|CallParentFunction OtherActor) ; This node is disabled and will not be called.\nDrag off pins to build functionality.
)

(event EventTick
  (params (DeltaSeconds :type Float%20%28single-precision%29))
  (|CallParentFunction DeltaSeconds) ; This node is disabled and will not be called.\nDrag off pins to build functionality.
)

(event EventTrigger
  (params (Player :type BP%20First%20Person%20Character%20Object%20Reference))
  (if (and (Variables|/Game/FirstPerson/Blueprints/BP_FirstPersonCharacter.BP_FirstPersonCharacter_C|GetbHasRifle Player) (Variables|/Game/FirstPerson/Blueprints/BP_FirstPersonCharacter.BP_FirstPersonCharacter_C|GetHasUniform Player))
    (Game|OpenLevel(byName) "Reality")))

(fn ConstructionScript
  (|CallParentFunction))