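; BP_Lock is a lock actor that opens a lock panel interface when triggered.
; If not yet opened, Trigger creates and shows a WBP_LockPannel widget, passes itself to it as the Lock, and shows the mouse cursor.
; It also disables input on the BP_FirstPersonCharacter through its CanInput flag while the panel is up; nothing here restores it or sets Opened.
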(event Collision|EventActorBeginOverlap
  (params (OtherActor :type Actor%20Object%20Reference))
  (|CallParentFunction OtherActor) ; This node is disabled and will not be called.\nDrag off pins to build functionality.
)

(event EventTick
  (params (DeltaSeconds :type Float%20%28single-precision%29))
  (|CallParentFunction DeltaSeconds) ; This node is disabled and will not be called.\nDrag off pins to build functionality.
)

(event EventTrigger
  (params (Player :type BP%20First%20Person%20Character%20Object%20Reference))
  (if (not (Variables|Default|GetOpened))
    (bind _returnvalue (UserInterface|CreateWidget "/Game/Blueprints/UI/WBP_LockPannel.WBP_LockPannel_C"))
    (Variables|Default|SetPanelUI _returnvalue)
    (UserInterface|Viewport|AddtoViewport _returnvalue 0)
    (Variables|/Script/Engine.PlayerController|SetbShowMouseCursor (Game|GetPlayerController 0) true)
    (Variables|/Game/Blueprints/UI/WBP_LockPannel.WBP_LockPannel_C|SetLock _returnvalue self)
    (bind _asbp_first_person_character (Utilities|Casting|CastToBP_FirstPersonCharacter (Game|GetPlayerCharacter 0)))
    (Variables|/Game/FirstPerson/Blueprints/BP_FirstPersonCharacter.BP_FirstPersonCharacter_C|SetCanInput _asbp_first_person_character false)))

(fn ConstructionScript
  (|CallParentFunction))