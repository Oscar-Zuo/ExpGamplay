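; BP_Uniform is a uniform pickup that lets the player put on a uniform.
; Its Trigger event sets HasUniform on the passed-in Player, sends a line saying Adam puts on his uniform to the BP_ChatGPTTester found in the level, then destroys the actor.
; BeginPlay, overlap and Tick are disabled stubs, so all behavior depends on Trigger being called.
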(event EventBeginPlay
  (|CallParentFunction) ; This node is disabled and will not be called.\nDrag off pins to build functionality.
)

(event Collision|EventActorBeginOverlap
  (params (OtherActor :type Actor%20Object%20Reference))
  (|CallParentFunction OtherActor) ; This node is disabled and will not be called.\nDrag off pins to build functionality.
)

(event EventTick
  (params (DeltaSeconds :type Float%20%28single-precision%29))
  (|CallParentFunction DeltaSeconds) ; This node is disabled and will not be called.\nDrag off pins to build functionality.
)

(event EventTrigger
  (params (Player :type BP%20First%20Person%20Character%20Object%20Reference))
  (Variables|/Game/FirstPerson/Blueprints/BP_FirstPersonCharacter.BP_FirstPersonCharacter_C|SetHasUniform Player true)
  (bind _returnvalue (Actor|GetActorOfClass "/Game/Blueprints/BP_ChatGPTTester.BP_ChatGPTTester_C"))
  (Default|SendMessage _returnvalue "G: Adam puts on his uniform.")
  (Actor|DestroyActor))

(fn ConstructionScript
  (|CallParentFunction))