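; Grabbable kebab interactor with three meat meshes that change appearance as they cook, exposing its stick as the grab component.
; The construction script gives each meat a dynamic material starting at the rare color.
; SetCookingStatus clamps the cooking value and lerps the color from rare to mid-well, then toward black past that threshold.
; It also sets the status that drives smoke particles, which grow denser and larger in the burning stage.
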(event EventBeginPlay)

(event Collision|EventActorBeginOverlap
  (params (OtherActor :type Actor%20Object%20Reference)))

(event EventTick
  (params (DeltaSeconds :type Float%20%28single-precision%29)))

(fn ConstructionScript
  (bind _foodmeshlist (LocalVariables|GetFoodMeshList))
  (Utilities|Array|Add _foodmeshlist (Variables|Default|GetMeat1))
  (Utilities|Array|Add _foodmeshlist (Variables|Default|GetMeat2))
  (Utilities|Array|Add _foodmeshlist (Variables|Default|GetMeat3))
  (for _array_element _foodmeshlist
    (bind _returnvalue (Rendering|Material|CreateDynamicMaterialInstance _array_element 0 "/Engine/BasicShapes/BasicShapeMaterial.BasicShapeMaterial" "None" :!class /Script/Engine.PrimitiveComponent))
    (Utilities|Array|Add (Variables|Default|GetFoodDynamicMaterialList) _returnvalue)
    (Rendering|Material|SetVectorParameterValue _returnvalue "Color" (Variables|Default|GetRareColor) :!class /Script/Engine.MaterialInstanceDynamic)))

(fn GetGrabableComponent
  (return (Variables|Default|GetStick)))

(fn SetCookingStatus
  (params (NewCookingStatus :type Float%20%28double-precision%29))
  (bind _totallyburnedvalue (Variables|Default|GetTotallyBurnedValue))
  (bind _fooddynamicmateriallist (Variables|Default|GetFoodDynamicMaterialList))
  (bind _returnvalue (Math|Float|Clamp(Float) NewCookingStatus 0.0 _totallyburnedvalue))
  (bind _output_get (Variables|Default|SetCookingStatus _returnvalue))
  (if (<= _returnvalue 1e+02)
    (for _array_element _fooddynamicmateriallist
      (Rendering|Material|SetVectorParameterValue _array_element "Color" (Math|Color|Lerp(LinearColor) (Variables|Default|GetRareColor) (Variables|Default|GetMidWellColor) (/ _output_get 1e+02)) :!class /Script/Engine.MaterialInstanceDynamic)
      (CallFunction|SetStatus 1))
    (else
      (for _array_element_2 _fooddynamicmateriallist
        (Rendering|Material|SetVectorParameterValue _array_element_2 "Color" (Math|Color|Lerp(LinearColor) (Variables|Default|GetMidWellColor) "(R=0.000000,G=0.000000,B=0.000000,A=1.000000)" (/ (- _output_get 1e+02) (Variables|Default|GetTotallyBurnedValue))) :!class /Script/Engine.MaterialInstanceDynamic)
        (CallFunction|SetStatus 2)))))

(fn SetParticleEffect
  (params (Status :type Integer))
  (bind _p_smoke (Variables|Default|GetP_Smoke))
  (switch int Status
    (:0
      (Components|Activation|Deactivate _p_smoke))
    (:1
      (Components|Activation|Activate _p_smoke false)
      (Effects|Components|ParticleSystem|SetFloatParameter _p_smoke "SpawnRate" 0.5)
      (Effects|Components|ParticleSystem|SetVectorParameter _p_smoke "Size" "0.500000,0.000000,0.000000"))
    (:2
      (Components|Activation|Activate _p_smoke false)
      (Effects|Components|ParticleSystem|SetFloatParameter _p_smoke "SpawnRate" 1.0)
      (Effects|Components|ParticleSystem|SetVectorParameter _p_smoke "Size" "1.000000,0.000000,0.000000"))))

(fn SetStatus
  (params (NewStatus :type Integer))
  (CallFunction|SetParticleEffect NewStatus))