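; A grabbable seasoning jar that seasons kebabs when the player shakes it.
; While held and moving above a velocity threshold, it tilts via the grabber's physics handle, plays a Niagara powder effect and enables an overlap collision.
; Overlapping kebabs are tracked in a list, and their season status rises each tick at a set speed.
; Slowing down or releasing it turns the powder and collision off.
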(event OnComponentBeginOverlap(SeasonCollision)
  (params (OverlappedComponent :type Primitive%20Component%20Object%20Reference) (OtherActor :type Actor%20Object%20Reference) (OtherComp :type Primitive%20Component%20Object%20Reference) (OtherBodyIndex :type Integer) (bFromSweep :type Boolean) (SweepResult :type Hit%20Result%20Structure%20%28by%20ref%29))
  (bind _asbp_kebab (Utilities|Casting|CastToBP_Kebab OtherActor))
  (Utilities|Set|Add (Variables|Default|GetSeasoning%20List) _asbp_kebab))

(event OnComponentEndOverlap(SeasonCollision)
  (params (OverlappedComponent :type Primitive%20Component%20Object%20Reference) (OtherActor :type Actor%20Object%20Reference) (OtherComp :type Primitive%20Component%20Object%20Reference) (OtherBodyIndex :type Integer))
  (bind _asbp_kebab (Utilities|Casting|CastToBP_Kebab OtherActor))
  (Utilities|Set|Remove (Variables|Default|GetSeasoning%20List) _asbp_kebab))

(event EventTick
  (params (DeltaSeconds :type Float%20%28single-precision%29))
  (bind _is_seasoning_function_enabled (Variables|Default|GetIs%20Seasoning%20Function%20Enabled))
  (bind _seasoning_list (Variables|Default|GetSeasoning%20List))
  (if (Variables|Default|GetIsGrabbed)
    (if (>= (Math|Vector|VectorLength (Transformation|GetVelocity)) (Variables|Default|GetMinumum%20Shake%20Velocity))
      (if _is_seasoning_function_enabled
        _
        (else
          (|EnableSeasonFunction)))
      (bind _result (Utilities|Set|ToArray _seasoning_list))
      (for _array_element _result
        (Utilities|IsValid _array_element
          (:Is%20Valid
            (Default|SetSeasonStatus _array_element (+ (* (Variables|Default|GetSeasoning%20Speed) DeltaSeconds) (Variables|/Game/Blueprints/Interactors/BP_Kebab.BP_Kebab_C|GetSeasonSatus _array_element))))
          (:Is%20Not%20Valid
            (Utilities|Set|Remove _seasoning_list _array_element))))
      (else
        (if _is_seasoning_function_enabled :!label _label
          (|DisableSeasonFunction))))
    (else
      (goto _label))))

(fn ConstructionScript
  (Collision|SetCollisionEnabled (Variables|Default|GetSeason%20Collision) "NoCollision"))

(fn GetGrabableComponent
  (return (Variables|Default|GetCylinder)))