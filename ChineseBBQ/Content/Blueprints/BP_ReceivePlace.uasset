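; BP_ReceivePlace is the delivery spot in the barbecue game, where kebabs are handed in to complete the first order.
; Its Box overlap tracks kebabs entering and leaving, comparing their count to the summed requirements of the GameState's first order.
; Once enough arrive, it collects their seasoning and cooking statuses, destroys them, and passes both lists to GameManager's FinishOrder.
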(event OnComponentBeginOverlap(Box)
  (params (OverlappedComponent :type Primitive%20Component%20Object%20Reference) (OtherActor :type Actor%20Object%20Reference) (OtherComp :type Primitive%20Component%20Object%20Reference) (OtherBodyIndex :type Integer) (bFromSweep :type Boolean) (SweepResult :type Hit%20Result%20Structure%20%28by%20ref%29))
  (bind _foodlist (Variables|Default|GetFoodList))
  (bind _cookvaluelist (Variables|Default|GetCookValueList))
  (bind _foodlist_2 (Variables|Default|GetFoodList))
  (bind _spicyvaluelist (Variables|Default|GetSpicyValueList))
  (bind _asbp_kebab (Utilities|Casting|CastToBP_Kebab OtherActor))
  (if (not (Utilities|Array|ContainsItem _foodlist _asbp_kebab))
    (Utilities|Array|Add _foodlist _asbp_kebab)
    (CallFunction|GetOrderTotalNum)
    (if (>= (Utilities|Array|Length _foodlist) (Variables|Default|GetOrderTotalNum))
      (for _array_element _foodlist_2
        (Utilities|Array|Add _spicyvaluelist (Variables|/Game/Blueprints/Interactors/BP_Kebab.BP_Kebab_C|GetSeasonSatus _array_element))
        (Utilities|Array|Add _cookvaluelist (Variables|/Game/Blueprints/Interactors/BP_Kebab.BP_Kebab_C|GetCookingStatus _array_element))
        (Actor|DestroyActor _array_element))
      (Utilities|Array|Clear _foodlist_2)
      (bind _outactors (Actor|GetAllActorsOfClass "/Script/ChineseBBQ.GameManager"))
      (Class|GameManager|FinishOrder (Utilities|Array|Get(acopy) _outactors) 0 _spicyvaluelist _cookvaluelist)
      (Utilities|Array|Clear _spicyvaluelist)
      (Utilities|Array|Clear _cookvaluelist))))

(event OnComponentEndOverlap(Box)
  (params (OverlappedComponent :type Primitive%20Component%20Object%20Reference) (OtherActor :type Actor%20Object%20Reference) (OtherComp :type Primitive%20Component%20Object%20Reference) (OtherBodyIndex :type Integer))
  (Utilities|Casting|CastToBP_Kebab OtherActor)
  (Utilities|Array|RemoveItem (Variables|Default|GetFoodList) 0))

(event EventBeginPlay
  (bind _aschinese_bbqgame_state (Utilities|Casting|CastToChineseBBQGameState (Game|GetGameState)))
  (Variables|Default|SetGame%20State _aschinese_bbqgame_state)
  (CallFunction|GetOrderTotalNum))

(event Collision|EventActorBeginOverlap
  (params (OtherActor :type Actor%20Object%20Reference)))

(event EventTick
  (params (DeltaSeconds :type Float%20%28single-precision%29)))

(fn ConstructionScript)

(fn GetOrderTotalNum
  (Variables|Default|SetOrderTotalNum 0)
  (bind _values (Utilities|Map|Values (.requirementsmap (Utilities|Array|Get(acopy) (Variables|/Script/ChineseBBQ.ChineseBBQGameState|GetorderList (Variables|Default|GetGame%20State))))))
  (for _array_element _values
    (Variables|Default|SetOrderTotalNum (+ _array_element (Variables|Default|GetOrderTotalNum)))))