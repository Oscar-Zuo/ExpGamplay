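; Spawn area for a Chinese BBQ game that keeps a kebab of a configurable type available at its location.
; BeginPlay spawns the first kebab at no cost, using the class's default scale.
; When a kebab leaves the Box and none of that type still overlaps it, a replacement spawns and 1 Money is deducted from ChineseBBQGameState.
; The InCD cooldown is checked, but the Delay logic that sets it is disconnected.
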(event OnComponentEndOverlap(Box)
  (params (OverlappedComponent :type Primitive%20Component%20Object%20Reference) (OtherActor :type Actor%20Object%20Reference) (OtherComp :type Primitive%20Component%20Object%20Reference) (OtherBodyIndex :type Integer))
  (bind _returnvalue (Transformation|GetActorTransform))
  (bind _kebabtype (Variables|Default|GetKebabType))
  (Utilities|Casting|CastToBP_Kebab OtherActor)
  (if (not (or (Utilities|Array|IsNotEmpty (Collision|GetOverlappingActors (Variables|Default|GetBox) _kebabtype :!class /Script/Engine.PrimitiveComponent)) (Variables|Default|GetInCD)))
    (Game|SpawnActorfromClass _kebabtype (Math|Transform|MakeTransform (.location _returnvalue) (.rotation _returnvalue) (.DefaultRootScale (Utilities|GetClassDefaults _kebabtype))) "AdjustIfPossibleButAlwaysSpawn" 0 0)
    (bind _aschinese_bbqgame_state (Utilities|Casting|CastToChineseBBQGameState (Game|GetGameState)))
    (Variables|/Script/ChineseBBQ.ChineseBBQGameState|Setmoney _aschinese_bbqgame_state (- (Variables|/Script/ChineseBBQ.ChineseBBQGameState|Getmoney _aschinese_bbqgame_state) 1.0))))

(event EventBeginPlay
  (bind _returnvalue (Transformation|GetActorTransform))
  (bind _kebabtype (Variables|Default|GetKebabType))
  (Game|SpawnActorfromClass _kebabtype (Math|Transform|MakeTransform (.location _returnvalue) (.rotation _returnvalue) (.DefaultRootScale (Utilities|GetClassDefaults _kebabtype))) "AdjustIfPossibleButAlwaysSpawn" 0 0))

(event EventTick
  (params (DeltaSeconds :type Float%20%28single-precision%29)))

(fn ConstructionScript)