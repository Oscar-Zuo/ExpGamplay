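; Enemy character that chases the third-person player across spherical planets, destroying number characters it touches and showing the game-over widget when it touches the player.
; Its movement component's tick is disabled for the first ten seconds of play.
; While gravity is active, Tick sets the gravity direction and feeds movement input toward the player.
; UpdatePlanetGravity selects a gravity center from overlapping BigSphere actors by distance, and helpers expose walk speed with a minimum clamp.
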(event OnComponentBeginOverlap(Collision)
  (params (OverlappedComponent :type Primitive%20Component%20Object%20Reference) (OtherActor :type Actor%20Object%20Reference) (OtherComp :type Primitive%20Component%20Object%20Reference) (OtherBodyIndex :type Integer) (bFromSweep :type Boolean) (SweepResult :type Hit%20Result%20Structure%20%28by%20ref%29))
  (Utilities|FlowControl|Sequence
    (:then_0
      (bind _asbp_base_number_character (Utilities|Casting|CastToBP_BaseNumberCharacter OtherActor))
      (Actor|DestroyActor _asbp_base_number_character))
    (:then_1
      (Utilities|Casting|CastToBP_ThirdPersonCharacter OtherActor)
      (bind _returnvalue (UserInterface|CreateWidget "/Game/UI/WBP_GameOver.WBP_GameOver_C"))
      (UserInterface|Viewport|AddtoViewport _returnvalue 0)
      (Variables|/Script/Engine.PlayerController|SetbShowMouseCursor (Game|GetPlayerController 0) true))))

(event EventBeginPlay
  (bind _charactermovement (Variables|Character|GetCharacterMovement))
  (Utilities|FlowControl|Sequence
    (:then_0
      (Components|Tick|SetComponentTickEnabled _charactermovement false)
      (Utilities|FlowControl|Delay 1e+01)
      (Components|Tick|SetComponentTickEnabled _charactermovement true))
    (:then_1
      (bind _asbp_third_person_character (Utilities|Casting|CastToBP_ThirdPersonCharacter (Game|Player|GetPlayerPawn 0)))
      (Variables|Default|SetPlayer _asbp_third_person_character))))

(event EventTick
  (params (DeltaSeconds :type Float%20%28single-precision%29))
  (if (Variables|Default|GetHasGravity)
    (Class|GravityMovementComponent|SetGravityDirection (Class|GravityCharacter|GetGravityMovementComponent) (Utilities|GetGravityDirectionInterp))
    (Class|PawnMovementComponent|AddInputVector (Variables|Character|GetCharacterMovement) (Math|Vector|Normalize (- (Transformation|GetActorLocation (Variables|Default|GetPlayer)) (Transformation|GetActorLocation))) false)))

(fn ConstructionScript)

(fn UpdatePlanetGravity
  (Variables|Default|SetHasGravity false)
  (for _array_element (Collision|GetOverlappingActors "/Script/PIRunner.BigSphere" :!class /Script/Engine.Actor)
    (bind _asbig_sphere (Utilities|Casting|CastToBigSphere _array_element))
    (if (<= (Math|Vector|VectorLength (- (Transformation|GetActorLocation _asbig_sphere) (Transformation|GetActorLocation))) (LocalVariables|GetDistance))
      (LocalVariables|SetLocation (Transformation|GetActorLocation _asbig_sphere))
      (LocalVariables|SetDistance (Math|Vector|VectorLength (- (Transformation|GetActorLocation _asbig_sphere) (Transformation|GetActorLocation))))
      (Variables|Default|SetHasGravity true)
      (Variables|/Script/Engine.CharacterMovementComponent|SetGravityScale (Variables|Character|GetCharacterMovement) 1.0)))
  (Variables|Default|SetCenterLocation (LocalVariables|GetLocation)))

(fn SetMoveSpeed
  (params (Speed :type Float%20%28double-precision%29))
  (Variables|/Script/Engine.CharacterMovementComponent|SetMaxWalkSpeed (Variables|Character|GetCharacterMovement) (Math|Float|Max(Float) Speed (Variables|Default|GetMinSpeed))))

(fn GetMoveSpeed
  (return (Variables|/Script/Engine.CharacterMovementComponent|GetMaxWalkSpeed (Variables|Character|GetCharacterMovement))))