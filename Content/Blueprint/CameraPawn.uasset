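; CameraPawn is a player camera pawn that views the BP_SmallBall and relays rotation input to the game.
; BeginPlay adds the Enhanced Input mapping context and caches the first BP_SmallBall found.
; IA_Rotate broadcasts its value to every BI_Movement actor through an interface message.
; IA_ChangeViewpoint toggles FollowBall, so each Tick either aims the spring arm at the ball or holds a fixed rotation.
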(event Input|EnhancedActionEvents|EnhancedInputActionIA_Rotate
  (params (ActionValue :type Vector%202D%20Structure) (ElapsedSeconds :type Float%20%28double-precision%29) (TriggeredSeconds :type Float%20%28double-precision%29) (InputAction :type Input%20Action%20Object%20Reference :default "/Game/Input/IA_Rotate.IA_Rotate"))
  (:Triggered
    (bind _outactors (Actor|GetAllActorswithInterface "/Game/Blueprint/BI_Movement.BI_Movement_C"))
    (for _array_element _outactors
      (Class|BIMovement|Rotate(Message) _array_element ActionValue))))

(event Input|EnhancedActionEvents|EnhancedInputActionIA_ChangeViewpoint
  (params (ActionValue :type Boolean) (ElapsedSeconds :type Float%20%28double-precision%29) (TriggeredSeconds :type Float%20%28double-precision%29) (InputAction :type Input%20Action%20Object%20Reference :default "/Game/Input/IA_ChangeViewpoint.IA_ChangeViewpoint"))
  (:Started
    (Variables|Default|SetFollow%20Ball (not (Variables|Default|GetFollow%20Ball)))))

(event EventBeginPlay
  (bind _asplayer_controller (Utilities|Casting|CastToPlayerController (Pawn|GetController)))
  (Input|AddMappingContext (PlayerController|LocalPlayerSubsystems|GetEnhancedInputLocalPlayerSubsystem _asplayer_controller) "/Game/Input/DefaultInput.DefaultInput" 0 "(bIgnoreAllPressedKeysUntilRelease=True,bForceImmediately=False)")
  (bind _returnvalue (Actor|GetActorOfClass "/Game/Blueprint/BP_SmallBall.BP_SmallBall_C"))
  (Utilities|IsValid _returnvalue
    (:Is%20Valid
      (Variables|Default|SetPlayer _returnvalue))))

(event Collision|EventActorBeginOverlap
  (params (OtherActor :type Actor%20Object%20Reference)))

(event EventTick
  (params (DeltaSeconds :type Float%20%28single-precision%29))
  (bind _player (Variables|Default|GetPlayer))
  (bind _springarm (Variables|Default|GetSpringArm))
  (if (Variables|Default|GetFollow%20Ball)
    (Utilities|IsValid _player
      (:Is%20Valid
        (Transformation|SetWorldRotation _springarm (.rotation (Class|KismetAnimationLibrary|Lookat (Transformation|GetActorTransform) (Transformation|GetActorLocation _player) "1.000000,0.000000,0.000000" false "0, 0, 0" 0.0)) false false)))
    (else
      (Transformation|SetWorldRotation _springarm "-90.000000,0.000000,0.000000" false false))))

(fn ConstructionScript)