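; BP_BigBall is a rotatable puzzle actor that the BP_SmallBall wins by reaching its end point while open.
; A Rotate event applies roll and pitch input as world rotation.
; Key pickups increment a count that, at the requirement, opens the end point, turning its light and dynamic glass material from red to green.
; SpringMove drives spring components along their forward vector with a timeline, disabling child box collision until the push finishes.
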(event OnComponentBeginOverlap(EndPoint)
  (params (OverlappedComponent :type Primitive%20Component%20Object%20Reference) (OtherActor :type Actor%20Object%20Reference) (OtherComp :type Primitive%20Component%20Object%20Reference) (OtherBodyIndex :type Integer) (bFromSweep :type Boolean) (SweepResult :type Hit%20Result%20Structure%20%28by%20ref%29))
  (Utilities|Casting|CastToBP_SmallBall OtherActor)
  (if (Variables|Default|GetIsOpen)
    (Development|PrintString "YOU WIN!")))

(event OnComponentBeginOverlap(Key)
  (params (OverlappedComponent :type Primitive%20Component%20Object%20Reference) (OtherActor :type Actor%20Object%20Reference) (OtherComp :type Primitive%20Component%20Object%20Reference) (OtherBodyIndex :type Integer) (bFromSweep :type Boolean) (SweepResult :type Hit%20Result%20Structure%20%28by%20ref%29))
  (Utilities|Casting|CastToBP_SmallBall OtherActor)
  (CallFunction|PickedKey)
  (Components|DestroyComponent (Variables|Default|GetKey)))

(event Custom|SpringMove
  (params (Component :type Static%20Mesh%20Component%20Object%20Reference) (Movement%20Scale :type Float%20%28double-precision%29))
  (bind _original_location (CallFunction|SpringPush Component))
  (bind _push (Timeline|PushTimeLine PlayFromStart)
    (:Update
      (Transformation|SetRelativeLocation Component (+ _original_location (* _push (Variables|Default|GetSpringLength) Movement%20Scale (Math|Vector|GetForwardVector (Variables|/Script/Engine.SceneComponent|GetRelativeRotation Component)))) false false))
    (:Finished
      (Transformation|SetRelativeLocation Component _original_location false false)
      (bind _asbox_collision (Utilities|Casting|CastToBoxComponent (Components|GetChildComponent Component 0)))
      (Collision|SetCollisionEnabled _asbox_collision "QueryAndPhysics"))))

(event EventBeginPlay
  (bind _sphere (Variables|Default|GetSphere))
  (bind _returnvalue (Rendering|Material|CreateDynamicMaterialInstance _sphere 0 (Rendering|Material|GetMaterial _sphere 0) "None" :!class /Script/Engine.PrimitiveComponent))
  (Variables|Default|SetEndPointMaterial _returnvalue)
  (CallFunction|SetEndPointStatus (Variables|Default|GetIsOpen)))

(event Collision|EventActorBeginOverlap
  (params (OtherActor :type Actor%20Object%20Reference)))

(event EventTick
  (params (DeltaSeconds :type Float%20%28single-precision%29)))

(event EventRotate
  (params (Input :type Vector%202D%20Structure))
  (Class|Actor|AddActorWorldRotation (Math|Rotator|MakeRotator (.x Input) (.y Input) 0.0)))

(fn ConstructionScript)

(fn PickedKey
  (bind _result (Math|Integer|IncrementInt (Variables|Default|GetKeyNum))
    (:%20%20
      (if (>= _result (Variables|Default|GetKeyRequirement))
        (CallFunction|SetEndPointStatus true)))))

(fn SetEndPointStatus
  (params (NewStatus :type Boolean))
  (bind _light (Variables|Default|GetLight))
  (bind _endpointmaterial (Variables|Default|GetEndPointMaterial))
  (if NewStatus
    (Rendering|Components|Light|SetLightColor _light "(R=0.000000,G=1.000000,B=0.000000,A=1.000000)" true)
    (Variables|Default|SetIsOpen true)
    (Rendering|Material|SetVectorParameterValue _endpointmaterial "ColorGlass" "(R=0.000000,G=1.000000,B=0.000000,A=1.000000)" :!class /Script/Engine.MaterialInstanceDynamic)
    (else
      (Rendering|Components|Light|SetLightColor _light "(R=1.000000,G=0.000000,B=0.000000,A=1.000000)" false)
      (Variables|Default|SetIsOpen false)
      (Rendering|Material|SetVectorParameterValue _endpointmaterial "ColorGlass" "(R=1.000000,G=0.000000,B=0.000000,A=1.000000)" :!class /Script/Engine.MaterialInstanceDynamic))))

(fn SpringPush
  (params (Cube :type Scene%20Component%20Object%20Reference))
  (bind _asbox_collision (Utilities|Casting|CastToBoxComponent (Components|GetChildComponent Cube 0))
    (:then
      (Collision|SetCollisionEnabled _asbox_collision "NoCollision"))
    (:CastFailed
      _))
  (return (Variables|/Script/Engine.SceneComponent|GetRelativeLocation Cube)))