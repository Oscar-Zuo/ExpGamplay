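; BP_BB3 is a rotatable ball-puzzle actor with five black holes, a key and a spring for BP_SmallBall.
; Each Tick, every black hole collision pulls overlapping balls toward it with a constant, mass-independent force.
; Touching a hole's Center teleports the ball to its original position and zeroes the actor's rotation.
; Ball overlaps also trigger PickedKey and destroy the key component, or fire SpringMove on the spring.
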(event OnComponentBeginOverlap(Center)
  (params (OverlappedComponent :type Primitive%20Component%20Object%20Reference) (OtherActor :type Actor%20Object%20Reference) (OtherComp :type Primitive%20Component%20Object%20Reference) (OtherBodyIndex :type Integer) (bFromSweep :type Boolean) (SweepResult :type Hit%20Result%20Structure%20%28by%20ref%29))
  (bind _asbp_small_ball (Utilities|Casting|CastToBP_SmallBall OtherActor))
  (Transformation|SetActorLocation _asbp_small_ball (Variables|/Game/Blueprint/BP_SmallBall.BP_SmallBall_C|GetOriginalPosition _asbp_small_ball) false true)
  (Transformation|SetActorRotation "0, 0, 0"))

(event OnComponentBeginOverlap(Center1)
  (params (OverlappedComponent :type Primitive%20Component%20Object%20Reference) (OtherActor :type Actor%20Object%20Reference) (OtherComp :type Primitive%20Component%20Object%20Reference) (OtherBodyIndex :type Integer) (bFromSweep :type Boolean) (SweepResult :type Hit%20Result%20Structure%20%28by%20ref%29))
  (bind _asbp_small_ball (Utilities|Casting|CastToBP_SmallBall OtherActor))
  (Transformation|SetActorLocation _asbp_small_ball (Variables|/Game/Blueprint/BP_SmallBall.BP_SmallBall_C|GetOriginalPosition _asbp_small_ball) false true)
  (Transformation|SetActorRotation "0, 0, 0"))

(event OnComponentBeginOverlap(Key1)
  (params (OverlappedComponent :type Primitive%20Component%20Object%20Reference) (OtherActor :type Actor%20Object%20Reference) (OtherComp :type Primitive%20Component%20Object%20Reference) (OtherBodyIndex :type Integer) (bFromSweep :type Boolean) (SweepResult :type Hit%20Result%20Structure%20%28by%20ref%29))
  (Utilities|Casting|CastToBP_SmallBall OtherActor)
  (CallFunction|PickedKey)
  (Components|DestroyComponent (Variables|Default|GetKey1)))

(event OnComponentBeginOverlap(SpringCollsion)
  (params (OverlappedComponent :type Primitive%20Component%20Object%20Reference) (OtherActor :type Actor%20Object%20Reference) (OtherComp :type Primitive%20Component%20Object%20Reference) (OtherBodyIndex :type Integer) (bFromSweep :type Boolean) (SweepResult :type Hit%20Result%20Structure%20%28by%20ref%29))
  (Utilities|Casting|CastToBP_SmallBall OtherActor)
  (CallFunction|SpringMove (Variables|Default|GetSpring1) 1.0))

(event OnComponentBeginOverlap(Center2)
  (params (OverlappedComponent :type Primitive%20Component%20Object%20Reference) (OtherActor :type Actor%20Object%20Reference) (OtherComp :type Primitive%20Component%20Object%20Reference) (OtherBodyIndex :type Integer) (bFromSweep :type Boolean) (SweepResult :type Hit%20Result%20Structure%20%28by%20ref%29))
  (bind _asbp_small_ball (Utilities|Casting|CastToBP_SmallBall OtherActor))
  (Transformation|SetActorLocation _asbp_small_ball (Variables|/Game/Blueprint/BP_SmallBall.BP_SmallBall_C|GetOriginalPosition _asbp_small_ball) false true)
  (Transformation|SetActorRotation "0, 0, 0"))

(event OnComponentBeginOverlap(Center3)
  (params (OverlappedComponent :type Primitive%20Component%20Object%20Reference) (OtherActor :type Actor%20Object%20Reference) (OtherComp :type Primitive%20Component%20Object%20Reference) (OtherBodyIndex :type Integer) (bFromSweep :type Boolean) (SweepResult :type Hit%20Result%20Structure%20%28by%20ref%29))
  (bind _asbp_small_ball (Utilities|Casting|CastToBP_SmallBall OtherActor))
  (Transformation|SetActorLocation _asbp_small_ball (Variables|/Game/Blueprint/BP_SmallBall.BP_SmallBall_C|GetOriginalPosition _asbp_small_ball) false true)
  (Transformation|SetActorRotation "0, 0, 0"))

(event OnComponentBeginOverlap(Center4)
  (params (OverlappedComponent :type Primitive%20Component%20Object%20Reference) (OtherActor :type Actor%20Object%20Reference) (OtherComp :type Primitive%20Component%20Object%20Reference) (OtherBodyIndex :type Integer) (bFromSweep :type Boolean) (SweepResult :type Hit%20Result%20Structure%20%28by%20ref%29))
  (bind _asbp_small_ball (Utilities|Casting|CastToBP_SmallBall OtherActor))
  (Transformation|SetActorLocation _asbp_small_ball (Variables|/Game/Blueprint/BP_SmallBall.BP_SmallBall_C|GetOriginalPosition _asbp_small_ball) false true)
  (Transformation|SetActorRotation "0, 0, 0"))

(event EventBeginPlay
  (bind _blackholelist (Variables|Default|GetBlackHoleList))
  (|CallParentFunction)
  (Utilities|Array|Add _blackholelist (Variables|Default|GetBlackHoleCollision))
  (Utilities|Array|Add _blackholelist (Variables|Default|GetBlackHoleCollision1))
  (Utilities|Array|Add _blackholelist (Variables|Default|GetBlackHoleCollision2))
  (Utilities|Array|Add _blackholelist (Variables|Default|GetBlackHoleCollision3))
  (Utilities|Array|Add _blackholelist (Variables|Default|GetBlackHoleCollision4)))

(event Collision|EventActorBeginOverlap
  (params (OtherActor :type Actor%20Object%20Reference))
  (|CallParentFunction OtherActor) ; This node is disabled and will not be called.\nDrag off pins to build functionality.
)

(event EventTick
  (params (DeltaSeconds :type Float%20%28single-precision%29))
  (|CallParentFunction DeltaSeconds)
  (for _array_element (Variables|Default|GetBlackHoleList)
    (for _array_element_2 (Collision|GetOverlappingActors _array_element "/Game/Blueprint/BP_SmallBall.BP_SmallBall_C" :!class /Script/Engine.PrimitiveComponent)
      (bind _asbp_small_ball (Utilities|Casting|CastToBP_SmallBall _array_element_2))
      (Physics|AddForce (Variables|/Game/Blueprint/BP_SmallBall.BP_SmallBall_C|GetSphere _asbp_small_ball) (* (Math|Vector|Normalize (- (Transformation|GetWorldLocation _array_element) (Transformation|GetActorLocation _array_element_2))) 9e+02) "None" true))))

(fn ConstructionScript
  (|CallParentFunction))